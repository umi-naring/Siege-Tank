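; Enemy tank Blueprint for the tank game, currently holding only per-frame debug logic.
; Each Tick prints the world locations of the ProjectileSpawnPoint and Cube components.
; It then sets SceneRoot's world location to the actor's location without sweep or teleport.
; The construction script is empty, and the graph contains no movement, aiming or firing logic.
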(event `self.ReceiveTick`
  (params (DeltaSeconds :type "Float (single-precision)"))
  (`KismetSystemLibrary.PrintString` (`KismetStringLibrary.Conv_VectorToString` (`SceneComponent.K2_GetComponentLocation` (`self.ProjectileSpawnPoint`))))
  (`KismetSystemLibrary.PrintString` (`KismetStringLibrary.Conv_VectorToString` (`SceneComponent.K2_GetComponentLocation` (`self.Cube`))))
  (`SceneComponent.K2_SetWorldLocation` (`self.SceneRoot`) (`self.K2_GetActorLocation`) false false))

(fn `UserConstructionScript`)